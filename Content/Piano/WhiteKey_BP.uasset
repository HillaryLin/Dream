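; WhiteKey_BP is a piano white key actor that plays its note and glows when the third-person character hits it.
; On BeginPlay it puts a dynamic instance of the white key material on the key mesh.
; A hit plays the Sound in 2D and runs a timeline that drives the material's Glow parameter.
; The construction script labels the key's text render with the Sound asset's name.
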(event OnComponentHit(Key_Mesh)
  (params (HitComponent :type Primitive%20Component%20Object%20Reference) (OtherActor :type Actor%20Object%20Reference) (OtherComp :type Primitive%20Component%20Object%20Reference) (NormalImpulse :type Vector :default "0, 0, 0") (Hit :type Hit%20Result%20Structure%20%28by%20ref%29))
  (Utilities|Casting|CastToThirdPersonCharacter OtherActor)
  (Audio|PlaySound2D (Variables|Default|GetSound) 1.0 1.0 0.0 0 0)
  (bind _newtrack_0 (Timeline|Timeline_0 PlayFromStart)
    (:Update
      (Rendering|Material|SetScalarParameterValue (stale EventBeginPlay _returnvalue) "Glow" _newtrack_0 :!class /Script/Engine.MaterialInstanceDynamic))))

(event EventBeginPlay
  (bind _key_mesh (Variables|Default|GetKey_Mesh))
  (bind _returnvalue (Rendering|Material|CreateDynamicMaterialInstance _key_mesh 0 "/Game/Piano/WhiteKey_MTL.WhiteKey_MTL" "None" :!class /Script/Engine.PrimitiveComponent))
  (Rendering|Material|SetMaterial _key_mesh 0 _returnvalue))

(fn ConstructionScript
  (Rendering|Components|TextRender|SetText (Variables|Default|GetTextRender) (Utilities|Text|ToText(String) (Utilities|GetObjectName (Variables|Default|GetSound)))))